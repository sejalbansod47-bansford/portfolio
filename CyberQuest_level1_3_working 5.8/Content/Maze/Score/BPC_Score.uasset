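; BPC_Score is a score component for the maze game that tracks the score and decides the win or loss.
; ScoreToAdd and ScoreToTakeaway both add their input to Score, so deductions need negative values, then call UpdateUIScore.
; UpdateUIScore pushes the score to the HUD on the first-person character, then checks fixed lower and upper limits, printing a lose or win message and opening the main menu level.
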(fn ScoretoAdd
  (params (ScoreToAdd :type Integer))
  (Variables|Default|SetScore (+ ScoreToAdd (Variables|Default|GetScore)))
  (CallFunction|UpdateUIScore))

(fn ScoretoTakeaway
  (params (ScoreToTakeaway :type Integer))
  (Variables|Default|SetScore (+ ScoreToTakeaway (Variables|Default|GetScore)))
  (CallFunction|UpdateUIScore))

(fn UpdateUIScore
  (bind _asbp_first_person_character_mine (Utilities|Casting|CastToBP_FirstPersonCharacter_Mine (Game|GetPlayerCharacter 0)))
  (Default|UpdateUI (Variables|/Game/Maze/FirstPerson/Blueprints/BP_FirstPersonCharacter_Mine.BP_FirstPersonCharacter_Mine_C|GetHud _asbp_first_person_character_mine) (Utilities|Text|ToText(Integer) (Variables|Default|GetScore)))
  (if (<= (Variables|Default|GetScore) -3)
    (Development|PrintString "You Lost :'(")
    (Game|OpenLevel(byName) "Mainmenulevel")
    (elif (>= (Variables|Default|GetScore) 7)
      (Development|PrintText "You won !!")
      (Game|OpenLevel(byName) "Mainmenulevel"))))