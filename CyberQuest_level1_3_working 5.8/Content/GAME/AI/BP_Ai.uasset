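; Enemy AI pawn that roams at random, chases pawns it sees and triggers game over on catching the player.
; Pawn sensing starts the chase, with a retriggerable delay returning it to roaming.
; A catch turns player and camera toward the AI, plays a montage, fades out, self-damages, shows game-over UI and pauses.
; A separate DealDamage event applies sphere-overlap damage with debug drawing.
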(event OnSeePawn(PawnSensing)
  (params (Pawn :type Pawn%20Object%20Reference))
  ;[0.15 0.15 0.15 0.5] Make AI chase you
  (Utilities|FlowControl|Sequence
    (:then_0
      (AI|AIMoveTo self "0, 0, 0" Pawn 5.0 false
        (:OnSuccess
          (CallFunction|CatchPlayer))))
    (:then_1
      (Utilities|FlowControl|RetriggerableDelay 1.0)
      (CallFunction|RandomRoam))))

(event OnComponentBeginOverlap(SphereOfDeath)
  (params (OverlappedComponent :type Primitive%20Component%20Object%20Reference) (OtherActor :type Actor%20Object%20Reference) (OtherComp :type Primitive%20Component%20Object%20Reference) (OtherBodyIndex :type Integer) (bFromSweep :type Boolean) (SweepResult :type Hit%20Result%20Structure%20%28by%20ref%29))
  ;[0.15 0.15 0.15 0.5] 🧩 Option 1: Use OnComponentBeginOverlap (Tried, did not work)
  (Utilities|Casting|CastToBP_ThirdPersonCharacter OtherActor))

(event Custom|Random%20Roam
  ;[0.15 0.15 0.15 0.5] Make AI chase you
  (AI|AIMoveTo self (.RandomLocation (AI|Navigation|GetRandomReachablePointinRadius (Transformation|GetActorLocation) 1.5e+03 0 0)) 0 5.0 false
    (:OnSuccess
      (CallFunction|RandomRoam))))

(event Custom|Catch%20Player
  (bind _returnvalue (Game|GetPlayerController 0))
  ;[0.15 0.15 0.15 0.5] face each other, fade screen and game over UI
  (Variables|Default|SetCaught? true)
  (Variables|Default|Setshould%20loop? true)
  (bind _asbp_third_person_character (Utilities|Casting|CastToBP_ThirdPersonCharacter (Game|GetPlayerCharacter 0)))
  (if (Variables|Default|Getshould%20loop?)
    (Utilities|FlowControl|Delay 0.001)
    (Transformation|SetActorRotation _asbp_third_person_character (Math|Interpolation|RInterpTo (Transformation|GetActorRotation _asbp_third_person_character) (Math|Rotator|FindLookatRotation (Transformation|GetActorLocation _asbp_third_person_character) (Transformation|GetActorLocation)) (Utilities|Time|GetWorldDeltaSeconds) 5.0))
    (Pawn|SetControlRotation _returnvalue (Math|Interpolation|RInterpTo (Pawn|GetControlRotation _returnvalue :!class /Script/Engine.Controller) (Math|Rotator|FindLookatRotation (Transformation|GetActorLocation _asbp_third_person_character) (Transformation|GetActorLocation)) (Utilities|Time|GetWorldDeltaSeconds) 5.0))
    (CallFunction|RotateLoop)
    (Utilities|FlowControl|DoOnce false :!label _label
      (:Completed
        (Utilities|FlowControl|Sequence
          (:then_0
            (Animation|PlayAnimMontage "/Game/GAME/AI/AM_Bot.AM_Bot" 1.0 "None")
            (Utilities|FlowControl|Delay 1.0)
            (CameraFades|StartCameraFade :self (Game|GetPlayerCameraManager 0) :ToAlpha 1.0 :Duration 1.5 :bShouldFadeAudio true :bHoldWhenFinished true)
            (Utilities|FlowControl|Delay 1.0)
            (Game|Damage|ApplyDamage self 1e+02 0 0 "/Script/Engine.DamageType")
            (bind _returnvalue_2 (UserInterface|CreateWidget "/Game/GAME/UI/WB_GameOver.WB_GameOver_C"))
            (UserInterface|Viewport|AddtoViewport _returnvalue_2 0)
            (Game|SetGamePaused true))
          (:then_1
            (Utilities|FlowControl|Delay 0.5)
            (Variables|Default|Setshould%20loop? false)
            (goto _label Reset)))))))

(event Custom|Rotate%20loop
  (bind _returnvalue (Game|GetPlayerController 0))
  ;[0.15 0.15 0.15 0.5] face each other, fade screen and game over UI
  (if (Variables|Default|Getshould%20loop?)
    (Utilities|FlowControl|Delay 0.001)
    (Transformation|SetActorRotation (stale Custom|Catch%20Player _asbp_third_person_character) (Math|Interpolation|RInterpTo (Transformation|GetActorRotation (stale Custom|Catch%20Player _asbp_third_person_character)) (Math|Rotator|FindLookatRotation (Transformation|GetActorLocation (stale Custom|Catch%20Player _asbp_third_person_character)) (Transformation|GetActorLocation)) (Utilities|Time|GetWorldDeltaSeconds) 5.0))
    (Pawn|SetControlRotation _returnvalue (Math|Interpolation|RInterpTo (Pawn|GetControlRotation _returnvalue :!class /Script/Engine.Controller) (Math|Rotator|FindLookatRotation (Transformation|GetActorLocation (stale Custom|Catch%20Player _asbp_third_person_character)) (Transformation|GetActorLocation)) (Utilities|Time|GetWorldDeltaSeconds) 5.0))
    (CallFunction|RotateLoop)
    (Utilities|FlowControl|DoOnce false :!label _label
      (:Completed
        (Utilities|FlowControl|Sequence
          (:then_0
            (Animation|PlayAnimMontage "/Game/GAME/AI/AM_Bot.AM_Bot" 1.0 "None")
            (Utilities|FlowControl|Delay 1.0)
            (CameraFades|StartCameraFade :self (Game|GetPlayerCameraManager 0) :ToAlpha 1.0 :Duration 1.5 :bShouldFadeAudio true :bHoldWhenFinished true)
            (Utilities|FlowControl|Delay 1.0)
            (Game|Damage|ApplyDamage self 1e+02 0 0 "/Script/Engine.DamageType")
            (bind _returnvalue_2 (UserInterface|CreateWidget "/Game/GAME/UI/WB_GameOver.WB_GameOver_C"))
            (UserInterface|Viewport|AddtoViewport _returnvalue_2 0)
            (Game|SetGamePaused true))
          (:then_1
            (Utilities|FlowControl|Delay 0.5)
            (Variables|Default|Setshould%20loop? false)
            (goto _label Reset)))))))

(event Custom|Deal%20Damage
  (bind _sphereofdeath (Variables|Default|GetSphereOfDeath))
  (bind _deathrange (Variables|Default|GetDeathRange))
  (bind _returnvalue (Transformation|GetWorldLocation _sphereofdeath))
  ;[0.15 0.15 0.15 0.5] Deal Damage
  (bind _outactors (Collision|SphereOverlapActors _returnvalue _deathrange (Utilities|Array|MakeArray "ObjectTypeQuery3") "/Script/Engine.Actor" (Utilities|Array|MakeArray self)))
  (Rendering|Debug|DrawDebugSphere _returnvalue _deathrange 12 "(R=1.000000,G=0.000000,B=0.000000,A=1.000000)" 2.0)
  (for _array_element _outactors
    (Game|Damage|ApplyDamage _array_element (Variables|Default|GetBase%20Damage) (Pawn|GetController) self "/Script/Engine.DamageType")))

(event EventBeginPlay
  ;[0.15 0.15 0.15 0.5] Make AI chase you
  (CallFunction|RandomRoam))

(fn ConstructionScript)