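; BP_Pickup is a collectible item whose mesh is chosen per instance through the construction script.
; Overlap volumes reveal DriveD, which turns to face the camera each tick, and toggle a WB_pickup widget created on BeginPlay.
; The player character entering TriggerBoxPickup calls CollectPickup on the BP_Shield_appear found in the level.
; A separate PickUp event shrinks the actor with a timeline, plays a sound and destroys it after a short delay.
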(event OnComponentBeginOverlap(Triggerboxpickup)
  (params (OverlappedComponent :type Primitive%20Component%20Object%20Reference) (OtherActor :type Actor%20Object%20Reference) (OtherComp :type Primitive%20Component%20Object%20Reference) (OtherBodyIndex :type Integer) (bFromSweep :type Boolean) (SweepResult :type Hit%20Result%20Structure%20%28by%20ref%29))
  (Utilities|Casting|CastToBP_ThirdPersonCharacter OtherActor)
  (bind _returnvalue (Actor|GetActorOfClass "/Game/GAME/Shield/BP_Shield_appear.BP_Shield_appear_C"))
  (Default|CollectPickup _returnvalue))

(event OnComponentBeginOverlap(triggertext)
  (params (OverlappedComponent :type Primitive%20Component%20Object%20Reference) (OtherActor :type Actor%20Object%20Reference) (OtherComp :type Primitive%20Component%20Object%20Reference) (OtherBodyIndex :type Integer) (bFromSweep :type Boolean) (SweepResult :type Hit%20Result%20Structure%20%28by%20ref%29))
  (Rendering|SetVisibility (Variables|Actor|GetDrive:%20D) true false))

(event OnComponentBeginOverlap(press'E'box)
  (params (OverlappedComponent :type Primitive%20Component%20Object%20Reference) (OtherActor :type Actor%20Object%20Reference) (OtherComp :type Primitive%20Component%20Object%20Reference) (OtherBodyIndex :type Integer) (bFromSweep :type Boolean) (SweepResult :type Hit%20Result%20Structure%20%28by%20ref%29))
  (Widget|SetVisibility (Variables|Default|GetPickup%20Widget%20Ref) "Visible"))

(event OnComponentEndOverlap(press'E'box)
  (params (OverlappedComponent :type Primitive%20Component%20Object%20Reference) (OtherActor :type Actor%20Object%20Reference) (OtherComp :type Primitive%20Component%20Object%20Reference) (OtherBodyIndex :type Integer))
  (Widget|SetVisibility (Variables|Default|GetPickup%20Widget%20Ref) "Hidden"))

(event EventPickUp
  (Development|PrintString "Item Picked")
  (bind _shrinktiimeline (Timeline|Shrink Play)
    (:Update
      (Transformation|SetWorldScale3D (Variables|Default|GetDefaultSceneRoot) (Math|Conversions|ToVector(Float) (Math|Float|Lerp 1.0 0.0 _shrinktiimeline)))
      (Utilities|FlowControl|DoOnce false
        (:Completed
          (Audio|PlaySound2D "/Engine/VREditor/Sounds/UI/Object_PickUp.Object_PickUp" 1.0 1.0 0.0 0 0)
          (Utilities|FlowControl|Delay 0.4)
          (Actor|DestroyActor))))))

(event EventTick
  (params (DeltaSeconds :type Float%20%28single-precision%29))
  (Transformation|SetWorldRotation (Variables|Actor|GetDrive:%20D) (Math|Rotator|FindLookatRotation (Transformation|GetWorldLocation (Variables|Actor|GetDrive:%20D)) (Transformation|GetActorLocation (Game|GetPlayerCameraManager 0))) false false))

(event EventBeginPlay
  (bind _returnvalue (UserInterface|CreateWidget "/Game/GAME/Pickup/WB_pickup.WB_pickup_C"))
  (bind _output_get (Variables|Default|SetPickup%20Widget%20Ref _returnvalue))
  (UserInterface|Viewport|AddtoViewport _output_get 0))

(fn ConstructionScript
  (Components|StaticMesh|SetStaticMesh (Variables|Default|GetPickup_object) (Variables|Default|GetBoxModelToPlace)))