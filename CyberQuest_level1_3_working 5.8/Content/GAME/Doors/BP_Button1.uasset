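; BP_Button1 is a proximity button that opens and closes BP_Door1, found in the level at BeginPlay.
; Box overlaps show and hide a 'Press F' widget, whose visibility also gates the OpenDoor event.
; OpenDoor alternates a timeline forward and backward through a FlipFlop, lerping the door's relative Z to lower or raise it.
; A DoOnce blocks retriggering until the timeline finishes.
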(event OnComponentBeginOverlap(Box)
  (params (OverlappedComponent :type Primitive%20Component%20Object%20Reference) (OtherActor :type Actor%20Object%20Reference) (OtherComp :type Primitive%20Component%20Object%20Reference) (OtherBodyIndex :type Integer) (bFromSweep :type Boolean) (SweepResult :type Hit%20Result%20Structure%20%28by%20ref%29))
  ;[0.15 0.15 0.15 0.5] UI--> Press 'F'
  (Widget|SetVisibility (Variables|Default|GetButton1%20Widget%20ref) "Visible"))

(event OnComponentEndOverlap(Box)
  (params (OverlappedComponent :type Primitive%20Component%20Object%20Reference) (OtherActor :type Actor%20Object%20Reference) (OtherComp :type Primitive%20Component%20Object%20Reference) (OtherBodyIndex :type Integer))
  ;[0.15 0.15 0.15 0.5] UI--> Press 'F'
  (Widget|SetVisibility (Variables|Default|GetButton1%20Widget%20ref) "Hidden"))

(event Custom|Open%20Door
  (if (Widget|IsVisible (Variables|Default|GetButton1%20Widget%20ref))
    (Utilities|FlowControl|DoOnce false :!label _label
      (:Completed
        (Utilities|FlowControl|FlipFlop
          (:A
            (bind _float_value (Timeline|Tiimeline_door_open PlayFromStart)
              (:Update
                (Transformation|SetRelativeLocation (Variables|/Game/GAME/Doors/BP_Door1.BP_Door1_C|GetDoor (Variables|Default|GetBP%20Door_1%20Ref)) (Math|Vector|MakeVector 0.0 0.0 (Math|Float|Lerp 0.0 -5e+02 _float_value)) false false))
              (:Finished
                (goto _label Reset))))
          (:B
            (Timeline|Tiimeline_door_open ReverseFromEnd)))))))

(event EventBeginPlay
  ;[0.15 0.15 0.15 0.5] UI--> Press 'F'
  (bind _returnvalue (UserInterface|CreateWidget "/Game/GAME/Doors/WB_F_Button.WB_F_Button_C"))
  (bind _output_get (Variables|Default|SetButton1%20Widget%20ref _returnvalue))
  (UserInterface|Viewport|AddtoViewport _output_get 0)
  (bind _returnvalue_2 (Actor|GetActorOfClass "/Game/GAME/Doors/BP_Door1.BP_Door1_C"))
  (Variables|Default|SetBP%20Door_1%20Ref _returnvalue_2))

(fn ConstructionScript)