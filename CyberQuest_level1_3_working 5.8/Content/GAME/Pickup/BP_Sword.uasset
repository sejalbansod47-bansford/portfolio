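; BP_Sword is a sword pickup whose mesh comes from SwModelToPlace in the construction script.
; Its trigger overlap toggles a pickup widget created at BeginPlay.
; PickupSw runs a timeline shrinking the root, with a DoOnce on its update that plays a sound, then destroys the actor after a delay.
; A Defender.exe component turns toward the camera each tick, shown on Sphere overlap and hidden when its own overlap ends.
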(event OnComponentBeginOverlap(Trigger_sword)
  (params (OverlappedComponent :type Primitive%20Component%20Object%20Reference) (OtherActor :type Actor%20Object%20Reference) (OtherComp :type Primitive%20Component%20Object%20Reference) (OtherBodyIndex :type Integer) (bFromSweep :type Boolean) (SweepResult :type Hit%20Result%20Structure%20%28by%20ref%29))
  (Widget|SetVisibility (Variables|Default|GetPickup_Wid_ref_sw) "Visible"))

(event OnComponentEndOverlap(Trigger_sword)
  (params (OverlappedComponent :type Primitive%20Component%20Object%20Reference) (OtherActor :type Actor%20Object%20Reference) (OtherComp :type Primitive%20Component%20Object%20Reference) (OtherBodyIndex :type Integer))
  (Widget|SetVisibility (Variables|Default|GetPickup_Wid_ref_sw) "Hidden"))

(event OnComponentBeginOverlap(Sphere)
  (params (OverlappedComponent :type Primitive%20Component%20Object%20Reference) (OtherActor :type Actor%20Object%20Reference) (OtherComp :type Primitive%20Component%20Object%20Reference) (OtherBodyIndex :type Integer) (bFromSweep :type Boolean) (SweepResult :type Hit%20Result%20Structure%20%28by%20ref%29))
  (Rendering|SetVisibility (Variables|Default|GetDefender.exe) true false))

(event OnComponentEndOverlap(Defender.exe)
  (params (OverlappedComponent :type Primitive%20Component%20Object%20Reference) (OtherActor :type Actor%20Object%20Reference) (OtherComp :type Primitive%20Component%20Object%20Reference) (OtherBodyIndex :type Integer))
  (Rendering|SetVisibility (Variables|Default|GetDefender.exe) false false))

(event EventBeginPlay
  (bind _returnvalue (UserInterface|CreateWidget "/Game/GAME/Pickup/WB_pickup.WB_pickup_C"))
  (bind _output_get (Variables|Default|SetPickup_Wid_ref_sw _returnvalue))
  (UserInterface|Viewport|AddtoViewport _output_get 0))

(event Collision|EventActorBeginOverlap
  (params (OtherActor :type Actor%20Object%20Reference)))

(event EventPickupSw
  (Development|PrintString "Item Picked")
  (bind _shrinktiimeline (Timeline|Timeline Play)
    (:Update
      (Transformation|SetWorldScale3D (Variables|Default|GetDefaultSceneRoot) (Math|Conversions|ToVector(Float) (Math|Float|Lerp 1.0 0.0 _shrinktiimeline)))
      (Utilities|FlowControl|DoOnce false
        (:Completed
          (Audio|PlaySound2D "/Engine/VREditor/Sounds/UI/Object_PickUp.Object_PickUp" 1.0 1.0 0.0 0 0)
          (Utilities|FlowControl|Delay 0.4)
          (Actor|DestroyActor))))))

(event EventTick
  (params (DeltaSeconds :type Float%20%28single-precision%29))
  (Transformation|SetWorldRotation (Variables|Default|GetDefender.exe) (Math|Rotator|FindLookatRotation (Transformation|GetWorldLocation (Variables|Default|GetDefender.exe)) (Transformation|GetActorLocation (Game|GetPlayerCameraManager 0))) false false))

(fn ConstructionScript
  (Components|StaticMesh|SetStaticMesh (Variables|Default|GetSword_model) (Variables|Default|GetSwModelToPlace)))