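; Shield actor that rises once enough pickups are collected and also hosts a game-over trigger.
; CollectPickup counts items and, at the maximum, waits before calling the bring-up event, whose FlipFlop plays or reverses a timeline moving the shield vertically.
; CyberShieldUp turns to face the player camera every tick.
; Player overlap with Game_over_collision shows the WB_ES widget; the game-pause node is unconnected.
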(event OnComponentBeginOverlap(Game_over_collision)
  (params (OverlappedComponent :type Primitive%20Component%20Object%20Reference) (OtherActor :type Actor%20Object%20Reference) (OtherComp :type Primitive%20Component%20Object%20Reference) (OtherBodyIndex :type Integer) (bFromSweep :type Boolean) (SweepResult :type Hit%20Result%20Structure%20%28by%20ref%29))
  (Utilities|Casting|CastToBP_ThirdPersonCharacter OtherActor)
  (bind _returnvalue (UserInterface|CreateWidget "/Game/GAME/Start_End_Screens/WB_ES.WB_ES_C"))
  (UserInterface|Viewport|AddtoViewport _returnvalue 0))

(event Custom|Bring-up%20Shield
  (Utilities|FlowControl|DoOnce false :!label _label
    (:Completed
      (Utilities|FlowControl|FlipFlop
        (:A
          (bind _shield_upliftment (Timeline|bring-up%20anim PlayFromStart)
            (:Update
              (Transformation|SetRelativeLocation (Variables|Default|GetShield) (Math|Vector|MakeVector 0.0 0.0 (Math|Float|Lerp 0.0 3.1e+02 _shield_upliftment)) true false))
            (:Finished
              (goto _label Reset))))
        (:B
          (Timeline|bring-up%20anim ReverseFromEnd))))))

(event Custom|Collect%20Pickup
  (bind _currentitemscollected (Variables|Default|GetcurrentItemsCollected))
  (Math|Integer|IncrementInt _currentitemscollected
    (:%20%20
      (if (>= _currentitemscollected (Variables|Default|GetmaxItemsCollected))
        (Utilities|FlowControl|DoOnce false
          (:Completed
            (Utilities|FlowControl|Delay 2e+01)
            (CallFunction|Bring-upShield)))))))

(event EventTick
  (params (DeltaSeconds :type Float%20%28single-precision%29))
  (Transformation|SetWorldRotation (Variables|Default|GetCyberShieldUp) (Math|Rotator|FindLookatRotation (Transformation|GetWorldLocation (Variables|Default|GetCyberShieldUp)) (Transformation|GetActorLocation (Game|GetPlayerCameraManager 0))) false false))

(fn ConstructionScript)